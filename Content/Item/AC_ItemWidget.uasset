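; Item component that builds a world-space widget showing its owning A_BaseItem's icon.
; CreateWidgetComponent adds a widget component to the owner, fills it with a W_ItemWidget and returns it.
; Uniform scale derives from the item's grid size, Offset aspect ratio and BaseSize, with the ratio factor capped at one.
; Rotation is fixed, and position is set in absolute world space from the origin, shifted by item size.
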(fn `CreateWidgetComponent`
  (returns (`Widget component` :type "WidgetComponent Object Reference"))
  (locals (BaseSize :type "Float (double-precision)" :default 5000.0))
  (bind _asa_base_item (cast `/Game/Item/A_BaseItem` (`self.GetOwner`)))
  (bind _returnvalue (`|AddComponentByClass` :`self` _asa_base_item :`Class` "/Script/UMG.WidgetComponent"))
  (bind (_details_name _details_size _details_mesh _details_physics _details_icon) (break `/Game/Structs/ItemStructure` (`/Game/Item/A_BaseItem.Details` _asa_base_item)))
  (bind _returnvalue_2 (`|CreateWidget` "/Game/Item/W_ItemWidget.W_ItemWidget_C" null _details_icon))
  (`WidgetComponent.SetWidget` _returnvalue _returnvalue_2)
  (`WidgetComponent.SetWidgetSpace` _returnvalue "World")
  (bind _returnvalue_3 (`KismetMathLibrary.Vector_GetAbs` (`/Game/Item/A_BaseItem.Offset` _asa_base_item)))
  (bind _details (`/Game/Item/A_BaseItem.Details` _asa_base_item))
  (bind (_returnvalue_x _returnvalue_y) (`KismetMathLibrary.BreakVector` (`KismetMathLibrary.MakeVector` (`KismetMathLibrary.Conv_IntToDouble` (break `/Game/Structs/IntSize` (`.Size_2_35D63ABA490A0B5C9DEFB9B555525C71` (break `/Game/Structs/ItemStructure` _details)))) (`KismetMathLibrary.Conv_IntToDouble` (`.length_6_0B08621E4AED037B168BD0AAB5A88426` (break `/Game/Structs/IntSize` (`.Size_2_35D63ABA490A0B5C9DEFB9B555525C71` (break `/Game/Structs/ItemStructure` _details))))))))
  (`SceneComponent.SetWorldScale3D` _returnvalue (`KismetMathLibrary.Conv_DoubleToVector` (* (`KismetMathLibrary.FClamp` (/ (/ (.x _returnvalue_3) (.y _returnvalue_3)) (`KismetMathLibrary.SafeDivide` (`KismetMathLibrary.Conv_IntToDouble` (break `/Game/Structs/IntSize` (`.Size_2_35D63ABA490A0B5C9DEFB9B555525C71` (break `/Game/Structs/ItemStructure` _details)))) (`KismetMathLibrary.Conv_IntToDouble` (`.length_6_0B08621E4AED037B168BD0AAB5A88426` (break `/Game/Structs/IntSize` (`.Size_2_35D63ABA490A0B5C9DEFB9B555525C71` (break `/Game/Structs/ItemStructure` _details)))))))) (/ (* (`KismetMathLibrary.SelectInt` (`KismetMathLibrary.Max` (break `/Game/Structs/IntSize` (`.Size_2_35D63ABA490A0B5C9DEFB9B555525C71` (break `/Game/Structs/ItemStructure` _details))) (`.length_6_0B08621E4AED037B168BD0AAB5A88426` (break `/Game/Structs/IntSize` (`.Size_2_35D63ABA490A0B5C9DEFB9B555525C71` (break `/Game/Structs/ItemStructure` _details))))) (`KismetMathLibrary.Min` (break `/Game/Structs/IntSize` (`.Size_2_35D63ABA490A0B5C9DEFB9B555525C71` (break `/Game/Structs/ItemStructure` _details))) (`.length_6_0B08621E4AED037B168BD0AAB5A88426` (break `/Game/Structs/IntSize` (`.Size_2_35D63ABA490A0B5C9DEFB9B555525C71` (break `/Game/Structs/ItemStructure` _details))))) (== (>= _returnvalue_x _returnvalue_y) (>= (.x _returnvalue_3) (.y _returnvalue_3)))) 50.0) (`local.BaseSize`)))))
  (`SceneComponent.K2_SetWorldRotation` _returnvalue (struct :`Pitch` 90.0) false false)
  (`SceneComponent.K2_SetWorldLocation` _returnvalue (+ (0.0 0.0 0.0) (* (`KismetMathLibrary.MakeVector` (`KismetMathLibrary.Conv_IntToDouble` (- 0 (break `/Game/Structs/IntSize` (`.Size_2_35D63ABA490A0B5C9DEFB9B555525C71` (break `/Game/Structs/ItemStructure` _details))))) (`KismetMathLibrary.Conv_IntToDouble` (`.length_6_0B08621E4AED037B168BD0AAB5A88426` (break `/Game/Structs/IntSize` (`.Size_2_35D63ABA490A0B5C9DEFB9B555525C71` (break `/Game/Structs/ItemStructure` _details)))))) 2.5)) false false)
  (return _returnvalue))