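; Inventory actor component that provides a grid mesh on its owning actor to represent the inventory's area.
; Init adds a static mesh component to the owner at a set offset and rotation, scaled by inventory width, length and cube scale.
; The grid material receives the width and length as "u" and "v" scalar parameters, and shadow casting is off.
; BeginPlay hides the stored grid component.
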(event `self.ReceiveBeginPlay`
  (`|ExecutionSequence`
    (:`then_1`
      (`SceneComponent.SetVisibility` (`self.GridComponent`) false false))))

(fn `Init`
  (locals (Transforms :type "Array of Transform Structure"))
  (bind (_size_width _size_length) (break `/Game/Structs/IntSize` (`self.Size`)))
  (bind (_size_width_2 _size_length_2) (break `/Game/Structs/IntSize` (`self.Size`)))
  (bind (_cubescale_x _cubescale_y) (`KismetMathLibrary.BreakVector` (`self.CubeScale`)))
  (bind _returnvalue (`|AddComponentByClass` (`self.GetOwner`) "/Script/Engine.StaticMeshComponent" false (`KismetMathLibrary.MakeTransform` (`self.Offset`) (`self.InventoryRotation`) (`KismetMathLibrary.MakeVector` (* (`KismetMathLibrary.Conv_IntToDouble` _size_width_2) _cubescale_x) (* (`KismetMathLibrary.Conv_IntToDouble` _size_length_2) _cubescale_y) 1.0))))
  (`StaticMeshComponent.SetStaticMesh` _returnvalue (`self.GridMesh`))
  (`PrimitiveComponent.SetMaterial` _returnvalue 0 (`self.Material`))
  (`MeshComponent.SetScalarParameterValueOnMaterials` _returnvalue "u" (`KismetMathLibrary.Conv_IntToDouble` _size_width))
  (`MeshComponent.SetScalarParameterValueOnMaterials` _returnvalue "v" (`KismetMathLibrary.Conv_IntToDouble` _size_length))
  (`PrimitiveComponent.SetCastShadow` _returnvalue false)
  (set `self.GridComponent` _returnvalue))